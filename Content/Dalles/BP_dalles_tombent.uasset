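; Falling floor tile that drops some time after a Character steps into its trigger box, then replaces itself.
; The box overlap starts a chain of timers with configurable delays, leading to the fall event that enables physics simulation on the cube.
; One second after falling starts, the actor destroys itself and spawns a new instance of its own class at its current transform.
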(event OnComponentBeginOverlap(Box)
  (params (OverlappedComponent :type Primitive%20Component%20Object%20Reference) (OtherActor :type Actor%20Object%20Reference) (OtherComp :type Primitive%20Component%20Object%20Reference) (OtherBodyIndex :type Integer) (bFromSweep :type Boolean) (SweepResult :type Hit%20Result%20Structure%20%28by%20ref%29))
  (Utilities|Casting|CastToCharacter OtherActor)
  (Utilities|Time|SetTimerbyEvent (EventDispatchers|CreateEvent :!event Custom|Temps) (Variables|Default|GetTime)))

(event Custom|Temps
  (Utilities|Time|SetTimerbyEvent (EventDispatchers|CreateEvent :!event Custom|DalleTombe) (Variables|Default|GetTime_0)))

(event Custom|DalleTombe
  (Physics|SetSimulatePhysics (Variables|Default|GetCube) true)
  (Utilities|FlowControl|Delay 1.0)
  (Actor|DestroyActor self)
  (Game|SpawnActorfromClass "BP_dalles_tombent_C" (Transformation|GetActorTransform) "Undefined" "OverrideRootScale" 0 0))

(event EventBeginPlay)

(event Collision|EventActorBeginOverlap
  (params (OtherActor :type Actor%20Object%20Reference)))

(event EventTick
  (params (DeltaSeconds :type Float%20%28single-precision%29)))

(fn ConstructionScript)