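; Patrolling police robot enemy whose spotlight color and speed follow player detection, and which can be hacked for points.
; A successful hack notifies its AI controller and unlocks the socketed battery, whose detachment ragdolls and unpossesses the robot.
; Dynamic materials and a camera-facing widget show hack affordability.
; Respawn replaces the actor with a fresh copy built from saved spawn and patrol info, unless permanently deactivated.
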(event Custom|OnLosePlayer
  ;[1 1 1] Couleur hacking GUI
  (Rendering|Components|Light|SetLightColor (Variables|Default|GetSpotLight) (Utilities|Struct|MakeLinearColor 1.0 1.0 1.0 0.0) true)
  (Variables|/Script/Engine.CharacterMovementComponent|SetMaxWalkSpeed (Variables|Character|GetCharacterMovement) (Variables|Speed|GetWalkSpeed)))

(event Custom|OnDetectPlayer
  ;[1 1 1] Couleur hacking GUI
  (Rendering|Components|Light|SetLightColor (Variables|Default|GetSpotLight) (Utilities|Struct|MakeLinearColor 1.0 0.0 0.0 0.0) true)
  (Variables|/Script/Engine.CharacterMovementComponent|SetMaxWalkSpeed (Variables|Character|GetCharacterMovement) (Variables|Speed|GetRunSpeed)))

(event Custom|On%20Sense%20Player
  ;[1 1 1] Couleur hacking GUI
  (Rendering|Components|Light|SetLightColor (Variables|Default|GetSpotLight) (Utilities|Struct|MakeLinearColor 1.0 1.0 0.0 0.0) true))

(event Custom|StartPatrolRoute
  ;[1 1 1] Événement qui permet de débuter la route de patrouille
  (bind _asaicontroller (Utilities|Casting|CastToAIController (Pawn|GetController)))
  (AI|Components|Blackboard|SetValueasObject (AI|GetBlackboard _asaicontroller) (Utilities|Name|MakeLiteralName "PatrolRoute") (Variables|PatrolRoute|GetPatrolRoute)))

(event Custom|DeactivateRobot
  ;[1 1 1] Désactivation d'un robot
  (Variables|Hacking|SetIsActive false)
  (Physics|SetSimulatePhysics (Variables|Character|GetMesh) true)
  (Collision|SetCollisionEnabled (Variables|Collision|GetCapsuleComponent) "NoCollision")
  (Rendering|SetVisibility (Variables|Default|GetSpotLight) false false)
  (Pawn|UnPossess (Pawn|GetController)))

(event Custom|OnRespawn
  (if (not (Variables|Hacking|GetIsPermentalyDeactivated))
    (Transformation|SetActorLocation "0.000000,0.000000,-1000.000000" false true)
    (bind _returnvalue (Game|SpawnActorfromClass "BP_RobotPolice_C" (.transform (Variables|Default|GetSpawnInfo)) "AlwaysSpawn" "MultiplyWithRoot" 0 0))
    (Variables|Default|SetRefToRespawnedRobot _returnvalue)
    (Variables|BP_RobotPolice_C|SetSpawnInfo (Variables|Default|GetRefToRespawnedRobot) (Variables|Default|GetSpawnInfo))
    (Variables|BP_RobotPolice_C|SetPatrolRoute (Variables|Default|GetRefToRespawnedRobot) (.patrolroute (Variables|Default|GetSpawnInfo)))
    (Variables|BP_RobotPolice_C|SetStartPatrolOnGameStart (Variables|Default|GetRefToRespawnedRobot) (.startpatrol (Variables|Default|GetSpawnInfo)))
    (Default|CallRespawed self)
    (Actor|DestroyActor)))

(event EventPossessed
  (params (NewController :type Controller%20Object%20Reference))
  (bind _self self)
  (bind _returnvalue (AI|GetAIController _self))
  (Utilities|IsValid _returnvalue
    (:Is%20Valid
      (Transformation|AttachComponentToComponent _returnvalue (Variables|Character|GetMesh) "Head" "KeepRelative" "KeepRelative" "KeepRelative" true)
      ;[1 1 1] Enregistre les informations importantes
      (Variables|Default|SetSpawnInfo (Utilities|Struct|MakeS_RobotSpawnInfo (Transformation|GetWorldTransform (Variables|Collision|GetCapsuleComponent)) (Variables|PatrolRoute|GetPatrolRoute) (Variables|PatrolRoute|GetStartPatrolOnGameStart))))))

(event EventBeginPlay
  (bind _mesh (Variables|Character|GetMesh))
  (bind _returnvalue (Transformation|GetSocketTransform _mesh "BatterySocket" "RTS_World"))
  ;[1 1 1] Begin Play
  (CallFunction|SetMaxWalkSpeed (Variables|Speed|GetWalkSpeed))
  ;[1 1 1] Spawn de la batterie
  (bind _returnvalue_2 (Game|SpawnActorfromClass "/Game/HackerZ/Blueprints/InteractableObjects/Blueprints/BP_Battery.BP_Battery_C" (Math|Transform|MakeTransform (.location _returnvalue) (.rotation _returnvalue) "1.000000,1.000000,1.000000") "AlwaysSpawn" "MultiplyWithRoot" self 0))
  (Variables|Default|SetBatteryRef _returnvalue_2)
  (EventDispatchers|AssignOnDetach _returnvalue_2 (delegate Custom|DeactivateRobot))
  (Transformation|AttachComponentToComponent (Variables|/Game/HackerZ/Blueprints/InteractableObjects/Blueprints/BP_Battery.BP_Battery_C|GetStaticMesh (Variables|Default|GetBatteryRef)) (Variables|Character|GetMesh) "BatterySocket" "KeepRelative" "KeepRelative" "KeepRelative" true)
  (Transformation|AttachComponentToComponent (Variables|/Game/HackerZ/Blueprints/InteractableObjects/Blueprints/BP_Battery.BP_Battery_C|GetScene (Variables|Default|GetBatteryRef)) (Variables|Collision|GetCapsuleComponent) "BatterySocket" "KeepWorld" "KeepWorld" "KeepRelative" true))

(event EventTick
  (params (DeltaSeconds :type Float%20%28single-precision%29))
  (bind _widget (Variables|Default|GetWidget))
  (CallFunction|UpdateMaterialHackDisplay)
  (Transformation|SetWorldRotation _widget (Math|Rotator|FindLookatRotation (Transformation|GetWorldLocation _widget) (Camera|GetCameraLocation (Game|GetPlayerCameraManager 0))) false false))

(fn ConstructionScript
  (bind _mesh (Variables|Character|GetMesh))
  (bind _returnvalue (Rendering|Material|CreateDynamicMaterialInstance _mesh 0 "/Game/HackerZ/Characters/Mannequins/Materials/Instances/Manny/MI_Manny_02.MI_Manny_02" "None" :!class /Script/Engine.PrimitiveComponent))
  (Variables|DynamicMaterials|SetMaterial2 _returnvalue)
  (bind _returnvalue_2 (Rendering|Material|CreateDynamicMaterialInstance _mesh 1 "/Game/HackerZ/Characters/Mannequins/Materials/Instances/Manny/MI_Manny_01.MI_Manny_01" "None" :!class /Script/Engine.PrimitiveComponent))
  (Variables|DynamicMaterials|SetMaterials1 _returnvalue_2))

(fn SetMaxWalkSpeed
  (params (MaxWalkSpeed :type Float%20%28double-precision%29))
  (Variables|/Script/Engine.CharacterMovementComponent|SetMaxWalkSpeed (Variables|Character|GetCharacterMovement) MaxWalkSpeed))

(fn Respawn
  ;[1 0 0.01909] Old, à retirer éventuellement
  (bind _returnvalue (Game|SpawnActorfromClass "BP_RobotPolice_C" (.transform (Variables|Default|GetSpawnInfo)) "AlwaysSpawn" "MultiplyWithRoot" 0 0))
  (Variables|BP_RobotPolice_C|SetSpawnInfo _returnvalue (Variables|Default|GetSpawnInfo))
  (Variables|BP_RobotPolice_C|SetPatrolRoute _returnvalue (.patrolroute (Variables|Default|GetSpawnInfo)))
  (Variables|BP_RobotPolice_C|SetStartPatrolOnGameStart _returnvalue (.startpatrol (Variables|Default|GetSpawnInfo))))

(fn UpdateMaterialHackDisplay
  (bind _widget (Variables|Default|GetWidget))
  (bind _output_get (Variables|DynamicMaterials|SetMaterialHackDisplay (Math|Interpolation|FInterpTo (Variables|DynamicMaterials|GetMaterialHackDisplay) 0.0 (Utilities|Time|GetWorldDeltaSeconds) 3.0)))
  (Rendering|Material|SetScalarParameterValue (Variables|DynamicMaterials|GetMaterial2) "DisplayHack" _output_get :!class /Script/Engine.MaterialInstanceDynamic)
  (if (>= (Variables|DynamicMaterials|GetMaterialHackDisplay) 1.0)
    (Development|SetHiddeninGame _widget false false)
    (else
      (Development|SetHiddeninGame _widget true false))))

(fn DisplayHackingGUI
  (params (PocketHacker :type BP%20Pocket%20Hacker%20SC%20Object%20Reference))
  (if (Variables|Hacking|GetIsActive)
    (bind _enough_ (Default|HasEnoughHackingPoints PocketHacker (Variables|Default|GetHackingPointsRequiredToHack)))
    (Rendering|Material|SetVectorParameterValue (Variables|DynamicMaterials|GetMaterial2) "DisplayHackingStatusColor" (Math|Color|SelectColor "(R=0.084637,G=1.000000,B=0.000000,A=1.000000)" "(R=1.000000,G=0.000000,B=0.000000,A=1.000000)" _enough_) :!class /Script/Engine.MaterialInstanceDynamic)
    (Variables|DynamicMaterials|SetMaterialHackDisplay 2.0)))

(fn GetHacked
  (params (HackTime :type Float%20%28double-precision%29) (PocketHacker :type BP%20Pocket%20Hacker%20SC%20Object%20Reference))
  (bind _self self)
  (bind _asai_controller_enemy (Utilities|Casting|CastToAI_Controller_Enemy (AI|GetAIController self)))
  (if (Variables|/Game/HackerZ/Blueprints/Enemy/AI/AI_Controller_Enemy.AI_Controller_Enemy_C|GetIsHacked _asai_controller_enemy)
    (return 0 false)
    (else
      (bind _isenoughpoints (Default|SpendHackingPoints PocketHacker (Variables|Default|GetHackingPointsRequiredToHack)))
      (if _isenoughpoints
        (Default|SetCanbeDisconnected (Variables|Default|GetBatteryRef) true)
        (bind _asai_controller_enemy_2 (Utilities|Casting|CastToAI_Controller_Enemy (AI|GetAIController _self)))
        (Variables|/Game/HackerZ/Blueprints/Enemy/AI/AI_Controller_Enemy.AI_Controller_Enemy_C|SetIsHacked _asai_controller_enemy_2 true)
        (Default|OnGetHacked _asai_controller_enemy_2 HackTime)
        (Development|PrintString "Got Hacked!")
        (Audio|PlaySoundatLocation "/Game/HackerZ/Blueprints/Enemy/Audio/Glitch_sound.Glitch_sound" (Transformation|GetActorLocation _self) "0, 0, 0" 0.5 1.0 0.0 0 0 0 0)
        (return self true)
        (else
          (Development|PrintString "Not enough hacking points to hack" true false "(R=1.000000,G=0.036710,B=0.000000,A=1.000000)")
          (return 0 false))))))

(fn ReturnHackingPointsRequired
  (return 0.0))