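; BP_TriggerStartPatrolRoute is a trigger that starts the patrol routes of a list of robot enemies when the player overlaps it.
; On BeginPlay it binds to each listed robot's respawn event.
; When a robot respawns, it swaps the old reference for the new robot, prints the removal result and rebinds, keeping the list valid across respawns.
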(event Custom|ReplaceRobotRef
  (params (RefToSelf :type BP%20Robot%20Police%20Object%20Reference))
  (bind _bp_enemylist (Variables|Default|GetBP_EnemyList))
  (bind _reftorespawnedrobot (Variables|/Game/HackerZ/Gameplay/Robots/BP_RobotPolice.BP_RobotPolice_C|GetRefToRespawnedRobot RefToSelf))
  (bind _returnvalue (Utilities|Array|RemoveItem _bp_enemylist RefToSelf))
  (Development|PrintString (Utilities|String|ToString(Boolean) _returnvalue))
  (Utilities|Array|AddUnique _bp_enemylist _reftorespawnedrobot)
  (EventDispatchers|BindEventtoRespawed _reftorespawnedrobot (delegate Custom|ReplaceRobotRef)))

(event EventBeginPlay
  (for _array_element (Variables|Default|GetBP_EnemyList)
    (EventDispatchers|BindEventtoRespawed _array_element (delegate Custom|ReplaceRobotRef))))

(event Collision|EventActorBeginOverlap
  (params (OtherActor :type Actor%20Object%20Reference))
  (Utilities|Casting|CastToBP_Player OtherActor)
  (for _array_element (Variables|Default|GetBP_EnemyList)
    (Default|StartPatrolRoute _array_element)))

(event EventTick
  (params (DeltaSeconds :type Float%20%28single-precision%29)))

(fn ConstructionScript)