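; HackerZ game mode that manages checkpoint saves, player death and respawn, level reload and quitting.
; Saving writes player location, health and rotation to a slot cleared on BeginPlay, and marks inactive BP_RobotPolice as permanently deactivated.
; Death restores that checkpoint and respawns player and robots, or reopens the level when no save exists.
; It also toggles AI perception debug on robot controllers and sets a windowed resolution in its construction script.
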(event Custom|OnDeath
  (bind _returnvalue (SaveGame|DoesSaveGameExist "CheckpointSave"))
  (if _returnvalue
    (CallFunction|OnLoadGame)
    (else
      (bind _returnvalue_2 (Game|GetCurrentLevelName true))
      (Game|OpenLevel(byName) (Utilities|String|StringToName _returnvalue_2)))))

(event Custom|ToggleDebugPerception
  ;[1 0.1355 0] Toggle débogue AI Perception
  (Utilities|FlowControl|FlipFlop
    (:A
      (bind _outactors (Actor|GetAllActorsOfClass "/Game/HackerZ/Gameplay/Robots/BP_RobotPolice.BP_RobotPolice_C"))
      (for _array_element _outactors
        (bind _asai_controller_enemy (Utilities|Casting|CastToAI_Controller_Enemy (AI|GetAIController _array_element)))
        (Variables|/Game/HackerZ/Blueprints/Enemy/AI/AI_Controller_Enemy.AI_Controller_Enemy_C|SetDebugPerception _asai_controller_enemy "ForOneFrame")))
    (:B
      (bind _outactors_2 (Actor|GetAllActorsOfClass "/Game/HackerZ/Gameplay/Robots/BP_RobotPolice.BP_RobotPolice_C"))
      (for _array_element_2 _outactors_2
        (bind _asai_controller_enemy_2 (Utilities|Casting|CastToAI_Controller_Enemy (AI|GetAIController _array_element_2)))
        (Variables|/Game/HackerZ/Blueprints/Enemy/AI/AI_Controller_Enemy.AI_Controller_Enemy_C|SetDebugPerception _asai_controller_enemy_2 "None")))))

(event Custom|OnSave
  (params (SaveLocation :type Vector) (SaveHealth :type Float%20%28double-precision%29) (SaveRotation :type Rotator))
  (bind _returnvalue (SaveGame|DoesSaveGameExist "CheckpointSave"))
  (if _returnvalue
    (bind _returnvalue_2 (SaveGame|LoadGamefromSlot "CheckpointSave"))
    (bind _asbp_save_game (Utilities|Casting|CastToBP_SaveGame _returnvalue_2)
      (:then
        (Variables|Default|SetSaveGame _asbp_save_game)
        (Variables|/Game/HackerZ/Blueprints/Player/FirstPersonBP/Blueprints/BP_SaveGame.BP_SaveGame_C|SetSaveLocation (Variables|Default|GetSaveGame) SaveLocation :!label _label)
        (Variables|/Game/HackerZ/Blueprints/Player/FirstPersonBP/Blueprints/BP_SaveGame.BP_SaveGame_C|SetSaveHealth (Variables|Default|GetSaveGame) SaveHealth)
        (Variables|/Game/HackerZ/Blueprints/Player/FirstPersonBP/Blueprints/BP_SaveGame.BP_SaveGame_C|SetSaveRotation (Variables|Default|GetSaveGame) SaveRotation)
        (bind _returnvalue_3 (SaveGame|SaveGametoSlot (Variables|Default|GetSaveGame) "CheckpointSave"))
        (Development|PrintString (Utilities|String|Append "Progress Saved : " (Utilities|String|ToString(Boolean) _returnvalue_3)))
        (bind _outactors (Actor|GetAllActorsOfClass "/Game/HackerZ/Gameplay/Robots/BP_RobotPolice.BP_RobotPolice_C"))
        (for _array_element _outactors
          (if (not (Variables|/Game/HackerZ/Gameplay/Robots/BP_RobotPolice.BP_RobotPolice_C|GetIsActive _array_element))
            (Variables|/Game/HackerZ/Gameplay/Robots/BP_RobotPolice.BP_RobotPolice_C|SetIsPermentalyDeactivated _array_element true))))
      (:CastFailed
        (Development|PrintString "Save Failed")))
    (else
      (bind _returnvalue_4 (SaveGame|CreateSaveGameObject "/Game/HackerZ/Blueprints/Player/FirstPersonBP/Blueprints/BP_SaveGame.BP_SaveGame_C"))
      (Variables|Default|SetSaveGame _returnvalue_4)
      (goto _label))))

(event Custom|OnLoadGame
  (bind _returnvalue (SaveGame|LoadGamefromSlot "CheckpointSave"))
  (bind _asbp_save_game (Utilities|Casting|CastToBP_SaveGame _returnvalue))
  (Variables|Default|SetBPSaveGame _asbp_save_game)
  (bind _asbp_player (Utilities|Casting|CastToBP_Player (Game|Player|GetPlayerPawn 0)))
  (Variables|Default|SetBPPlayer _asbp_player)
  (Utilities|FlowControl|Sequence
    (:then_0
      ;[1 1 1] Reset Player position and Health
      (Transformation|SetActorLocation (Variables|Default|GetBPPlayer) (Variables|/Game/HackerZ/Blueprints/Player/FirstPersonBP/Blueprints/BP_SaveGame.BP_SaveGame_C|GetSaveLocation (Variables|Default|GetBPSaveGame)) false false))
    (:then_1
      (Variables|/Game/HackerZ/Blueprints/Player/BP_Player.BP_Player_C|SetHealthCurrent (Variables|Default|GetBPPlayer) (Variables|/Game/HackerZ/Blueprints/Player/FirstPersonBP/Blueprints/BP_SaveGame.BP_SaveGame_C|GetSaveHealth (Variables|Default|GetBPSaveGame))))
    (:then_2
      (Pawn|SetControlRotation (Pawn|GetController (Variables|Default|GetBPPlayer)) (Variables|/Game/HackerZ/Blueprints/Player/FirstPersonBP/Blueprints/BP_SaveGame.BP_SaveGame_C|GetSaveRotation (Variables|Default|GetBPSaveGame))))
    (:then_3
      (bind _outactors (Actor|GetAllActorsOfClass "/Game/HackerZ/Gameplay/Robots/BP_RobotPolice.BP_RobotPolice_C"))
      (for _array_element _outactors
        (Default|OnRespawn _array_element)))
    (:then_4
      (Default|OnRespawn (Variables|Default|GetBPPlayer)))))

(event Custom|OnReloadLevel
  (SaveGame|DeleteGameinSlot "CheckpointSave")
  (bind _returnvalue (Game|GetCurrentLevelName true))
  (Game|OpenLevel(byName) (Utilities|String|StringToName _returnvalue)))

(event Custom|QuitGame
  (Game|QuitGame 0 "Quit" false))

(event EventBeginPlay
  (Development|PrintString "Game On")
  (SaveGame|DeleteGameinSlot "CheckpointSave"))

(fn ConstructionScript
  (bind _returnvalue (Settings|GetGameUserSettings))
  (Class|GameUserSettings|SetFullscreenMode _returnvalue "Windowed")
  (Class|GameUserSettings|SetScreenResolution _returnvalue (Utilities|Struct|MakeIntPoint 3840 1080)))