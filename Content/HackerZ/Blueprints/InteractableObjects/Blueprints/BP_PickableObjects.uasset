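; BP_PickableObjects is a pickup actor that the player collects by touching it.
; On overlap it passes its Pickable, Data and itself to BP_Player's OnPickup.
; Its own OnPickUp event plays a pickup sound at its location and destroys the actor.
; Tick animates the Scene component with a delta-time yaw spin and a sine-wave vertical bob, both tuned by multiplier variables.
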(event Custom|OnPickUp
  (Audio|PlaySoundatLocation "/Game/HackerZ/Blueprints/InteractableObjects/Audio/PickUp_sound.PickUp_sound" (Transformation|GetActorLocation) "0, 0, 0" 1.0 1.0 0.0 0 0 0 0)
  (Actor|DestroyActor))

(event Collision|EventActorBeginOverlap
  (params (OtherActor :type Actor%20Object%20Reference))
  (bind _asbp_player (Utilities|Casting|CastToBP_Player OtherActor))
  (Default|OnPickup _asbp_player (Variables|Default|GetPickable) (Variables|Default|GetData) self))

(event EventTick
  (params (DeltaSeconds :type Float%20%28single-precision%29))
  (bind _scene (Variables|Default|GetScene))
  ;[1 1 1] Animation de l'objet
  (Transformation|SetRelativeRotation _scene (Math|Rotator|MakeRotator 0.0 0.0 (Math|Float|%(Float) (+ (.yaw (Variables|/Script/Engine.SceneComponent|GetRelativeRotation _scene)) (* (Utilities|Time|GetWorldDeltaSeconds) (Variables|Default|GetRotationMultiplier))) 3.6e+02)) false false)
  (Transformation|SetRelativeLocation _scene (Math|Vector|MakeVector 0.0 0.0 (* (Math|Trig|Sin(Radians) (* (Utilities|Time|GetTimeSeconds) (Variables|Default|GetAnimationSpeedMultiplier))) (Variables|Default|GetAnimationAmplitudeMultiplier))) false false))

(fn ConstructionScript)